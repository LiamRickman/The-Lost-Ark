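; BP_Exit is the level exit, blocked until the player collects the idol.
; Tick polls the FirstPersonCharacter's IdolCollected flag, then hides the blocking cubes, disables their collision and lights a spotlight.
; The InRange trigger shows cannot-enter text while the idol is missing.
; ExitCheck overlap shows the win HUD and pauses, setting GamePaused on the character cached by InRange without filtering the overlapping actor.
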(event OnComponentBeginOverlap(InRange)
  (params (OverlappedComponent :type Primitive%20Component%20Object%20Reference) (OtherActor :type Actor%20Object%20Reference) (OtherComp :type Primitive%20Component%20Object%20Reference) (OtherBodyIndex :type Integer) (bFromSweep :type Boolean) (SweepResult :type Hit%20Result%20Structure%20%28by%20ref%29))
  ;[1 1 1] Show cannot enter text
  (bind _asfirst_person_character (Utilities|Casting|CastToFirstPersonCharacter OtherActor))
  (if (not (Variables|/Game/Level/Blueprints/Character/FirstPersonCharacter.FirstPersonCharacter_C|GetIdolCollected _asfirst_person_character))
    (Rendering|SetVisibility (Variables|Default|GetTextRender) true false)))

(event OnComponentEndOverlap(InRange)
  (params (OverlappedComponent :type Primitive%20Component%20Object%20Reference) (OtherActor :type Actor%20Object%20Reference) (OtherComp :type Primitive%20Component%20Object%20Reference) (OtherBodyIndex :type Integer))
  ;[1 1 1] Hide cannot enter text
  (Rendering|SetVisibility (Variables|Default|GetTextRender) false false))

(event OnComponentBeginOverlap(ExitCheck)
  (params (OverlappedComponent :type Primitive%20Component%20Object%20Reference) (OtherActor :type Actor%20Object%20Reference) (OtherComp :type Primitive%20Component%20Object%20Reference) (OtherBodyIndex :type Integer) (bFromSweep :type Boolean) (SweepResult :type Hit%20Result%20Structure%20%28by%20ref%29))
  ;[1 1 1] Pause game and show end win HUD
  (Viewport|RemoveAllWidgets)
  (bind _returnvalue (UserInterface|CreateWidget "/Game/Level/Blueprints/HUD/HUD_GameEnd_Win.HUD_GameEnd_Win_C"))
  (UserInterface|Viewport|AddtoViewport _returnvalue 0)
  (Variables|/Script/Engine.PlayerController|SetbShowMouseCursor (Game|GetPlayerController 0) true)
  (Variables|/Game/Level/Blueprints/Character/FirstPersonCharacter.FirstPersonCharacter_C|SetGamePaused (stale OnComponentBeginOverlap(InRange) _asfirst_person_character) true)
  (Game|SetGamePaused true))

(event EventTick
  (params (DeltaSeconds :type Float%20%28single-precision%29))
  (bind _cube (Variables|Default|GetCube))
  ;[1 1 1] Check if idol has been collected
  (bind _asfirst_person_character (Utilities|Casting|CastToFirstPersonCharacter (Game|GetPlayerCharacter 0)))
  (if (Variables|/Game/Level/Blueprints/Character/FirstPersonCharacter.FirstPersonCharacter_C|GetIdolCollected _asfirst_person_character)
    (Rendering|SetVisibility _cube false false)
    (Collision|SetCollisionEnabled _cube "NoCollision")
    (Rendering|SetVisibility (Variables|Default|GetSpotLight) true false)))

(fn ConstructionScript)