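; BP_Text is a placeable world text actor that can reveal itself when the player comes close.
; On BeginPlay it applies its DisplayText, TextMaterial and TextColour variables to the Text render component.
; Unless AlwaysVisible is set, overlaps on the InRange component show the text when the player character enters and hide it when they leave.
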(event OnComponentBeginOverlap(InRange)
  (params (OverlappedComponent :type Primitive%20Component%20Object%20Reference) (OtherActor :type Actor%20Object%20Reference) (OtherComp :type Primitive%20Component%20Object%20Reference) (OtherBodyIndex :type Integer) (bFromSweep :type Boolean) (SweepResult :type Hit%20Result%20Structure%20%28by%20ref%29))
  ;[1 1 1] Show text when close
  (if (not (Variables|Default|GetAlwaysVisible))
    (if (== OtherActor (Game|GetPlayerCharacter 0))
      (Rendering|SetVisibility (Variables|Default|GetText) true false))))

(event OnComponentEndOverlap(InRange)
  (params (OverlappedComponent :type Primitive%20Component%20Object%20Reference) (OtherActor :type Actor%20Object%20Reference) (OtherComp :type Primitive%20Component%20Object%20Reference) (OtherBodyIndex :type Integer))
  ;[1 1 1] Show text when close
  (if (not (Variables|Default|GetAlwaysVisible))
    (if (== OtherActor (Game|GetPlayerCharacter 0))
      (Rendering|SetVisibility (Variables|Default|GetText) false false))))

(event EventBeginPlay
  (bind _text (Variables|Default|GetText))
  ;[1 1 1] Setting text values
  (Rendering|Components|TextRender|SetText (Variables|Default|GetText) (Utilities|Text|ToText(String) (Variables|Default|GetDisplayText)))
  (Rendering|Material|SetMaterial _text 0 (Variables|Default|GetTextMaterial))
  (Rendering|Components|TextRender|SetTextRenderColor _text (Variables|Default|GetTextColour)))

(fn ConstructionScript)