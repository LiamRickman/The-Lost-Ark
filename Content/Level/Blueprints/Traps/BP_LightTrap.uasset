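; Light trap actor that fires an arrow when the player overlaps its light collision.
; When movement is enabled, a timeline carries the whole actor along a referenced route spline.
; The overlap plays a sound and moves the arrow and its collision in parallel to an endpoint, then back after a delay.
; Arrow hits call Damage on the first-person character, gated by a DoOnce that resets after a short delay.
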(event OnComponentBeginOverlap(LightCollision)
  (params (OverlappedComponent :type Primitive%20Component%20Object%20Reference) (OtherActor :type Actor%20Object%20Reference) (OtherComp :type Primitive%20Component%20Object%20Reference) (OtherBodyIndex :type Integer) (bFromSweep :type Boolean) (SweepResult :type Hit%20Result%20Structure%20%28by%20ref%29))
  (bind _arrowstart (Variables|Default|GetArrowStart))
  (bind _arrowrotation (Variables|Default|GetArrowRotation))
  (bind _arrow (Variables|Default|GetArrow))
  (bind _arrowend (Variables|Default|GetArrowEnd))
  (bind _arrow_collision (Variables|Default|GetArrow_Collision))
  (bind _arrowspeed (Variables|Default|GetArrowSpeed))
  ;[1 1 1] Fire/Reset Arrow
  (if (== OtherActor (Game|GetPlayerCharacter 0))
    (Utilities|FlowControl|Sequence
      (:then_0
        (Audio|PlaySoundatLocation "/Game/Level/Audio/Arrow.Arrow" (Variables|Default|GetArrowEnd) "0, 0, 0" 1.0 1.0 0.0 0 0 0)
        (Components|MoveComponentTo _arrow _arrowend _arrowrotation false false _arrowspeed false)
        (Utilities|FlowControl|Delay 1.0)
        (Components|MoveComponentTo _arrow _arrowstart _arrowrotation false false _arrowspeed false))
      (:then_1
        (Components|MoveComponentTo _arrow_collision _arrowend _arrowrotation false false _arrowspeed false)
        (Utilities|FlowControl|Delay 1.0)
        (Components|MoveComponentTo _arrow_collision _arrowstart _arrowrotation false false _arrowspeed false)))))

(event OnComponentBeginOverlap(Arrow_Collision)
  (params (OverlappedComponent :type Primitive%20Component%20Object%20Reference) (OtherActor :type Actor%20Object%20Reference) (OtherComp :type Primitive%20Component%20Object%20Reference) (OtherBodyIndex :type Integer) (bFromSweep :type Boolean) (SweepResult :type Hit%20Result%20Structure%20%28by%20ref%29))
  ;[1 1 1] Hit by arrow
  (bind _asfirst_person_character (Utilities|Casting|CastToFirstPersonCharacter OtherActor))
  (Variables|Default|SetInVolume true)
  (Utilities|FlowControl|DoOnce false :!label _label
    (:Completed
      (Default|Damage _asfirst_person_character)
      (if (Variables|Default|GetInVolume)
        (Utilities|FlowControl|Delay 2.0)
        (goto _label Reset)))))

(event Custom|MoveLight
  (bind _routeref (Variables|Default|GetRouteRef))
  (bind _lightroute (Variables|/Game/Level/Blueprints/Traps/BP_LightTrap_Route.BP_LightTrap_Route_C|GetLightRoute _routeref))
  ;[1 1 1] Move light
  (Components|Timeline|SetPlayRate (Variables|Default|GetLightMover) (/ 1.0 (Variables|Default|GetMoveSpeed)))
  (bind _alpha (Timeline|LightMover Play)
    (:Update
      (Variables|Default|SetAlpha _alpha)
      (Transformation|SetActorLocationAndRotation (Spline|GetLocationatDistanceAlongSpline _lightroute (Math|Float|Lerp 0.0 (Spline|GetSplineLength _lightroute) (Variables|Default|GetAlpha)) "World") (Spline|GetRotationatDistanceAlongSpline _lightroute (Math|Float|Lerp 0.0 (Spline|GetSplineLength _lightroute) (Variables|Default|GetAlpha)) "World")))))

(event EventBeginPlay
  ;[1 1 1] Set Variables / Check if moving
  (Variables|Default|SetArrowStart (Variables|/Script/Engine.SceneComponent|GetRelativeLocation (Variables|Default|GetArrow)))
  (Variables|Default|SetArrowEnd (Variables|/Script/Engine.SceneComponent|GetRelativeLocation (Variables|Default|GetArrow_Endpoint)))
  (Variables|Default|SetArrowRotation (Transformation|GetWorldRotation (Variables|Default|GetArrow)))
  (if (Variables|Default|GetMoveTrue)
    (CallFunction|MoveLight)))

(fn ConstructionScript)