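; Floor trap that shoots spikes when the player character steps on its pressure plate and damages a first-person character they touch.
; Plate overlap moves the spike and its collision to an endpoint captured at BeginPlay, then returns both after a short delay.
; Spike overlap calls Damage on the character through a DoOnce that resets after a cooldown while InVolume is true, a flag never cleared here.
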(event OnComponentBeginOverlap(Plate_Collision)
  (params (OverlappedComponent :type Primitive%20Component%20Object%20Reference) (OtherActor :type Actor%20Object%20Reference) (OtherComp :type Primitive%20Component%20Object%20Reference) (OtherBodyIndex :type Integer) (bFromSweep :type Boolean) (SweepResult :type Hit%20Result%20Structure%20%28by%20ref%29))
  (bind _spike (Variables|Default|GetSpike))
  (bind _spikeend (Variables|Default|GetSpikeEnd))
  (bind _spike_collision (Variables|Default|GetSpike_Collision))
  (bind _speed (Variables|Default|GetSpeed))
  (bind _spikestart (Variables|Default|GetSpikeStart))
  ;[1 1 1] Colliding with Plate
  (if (== OtherActor (Game|GetPlayerCharacter 0))
    (Utilities|FlowControl|Sequence
      (:then_0
        (Components|MoveComponentTo _spike _spikeend "0, 0, 0" false false _speed false)
        (Utilities|FlowControl|Delay 1.0)
        (Components|MoveComponentTo _spike _spikestart "0, 0, 0" false false _speed false))
      (:then_1
        (Components|MoveComponentTo _spike_collision _spikeend "0, 0, 0" false false _speed false)
        (Utilities|FlowControl|Delay 1.0)
        (Components|MoveComponentTo _spike_collision _spikestart "0, 0, 0" false false _speed false)))))

(event OnComponentBeginOverlap(Spike_Collision)
  (params (OverlappedComponent :type Primitive%20Component%20Object%20Reference) (OtherActor :type Actor%20Object%20Reference) (OtherComp :type Primitive%20Component%20Object%20Reference) (OtherBodyIndex :type Integer) (bFromSweep :type Boolean) (SweepResult :type Hit%20Result%20Structure%20%28by%20ref%29))
  ;[1 1 1] Colliding with Spike
  (bind _asfirst_person_character (Utilities|Casting|CastToFirstPersonCharacter OtherActor))
  (Variables|Default|SetInVolume true)
  (Utilities|FlowControl|DoOnce false :!label _label
    (:Completed
      (Default|Damage _asfirst_person_character)
      (if (Variables|Default|GetInVolume)
        (Utilities|FlowControl|Delay 2.0)
        (goto _label Reset)))))

(event EventBeginPlay
  ;[1 1 1] Set Locations
  (Variables|Default|SetSpikeStart (Variables|/Script/Engine.SceneComponent|GetRelativeLocation (Variables|Default|GetSpike)))
  (Variables|Default|SetSpikeEnd (Variables|/Script/Engine.SceneComponent|GetRelativeLocation (Variables|Default|GetSpike_Endpoint))))

(fn ConstructionScript)