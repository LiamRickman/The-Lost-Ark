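; Indiana Jones-style boulder trap that rolls along a spline route once the player has collected the idol and enters the StartMoveCheck trigger.
; Tick caches the player character's idol state for that trigger check.
; MoveBoulder plays a crumble sound, waits, then runs a speed-scaled timeline setting location and rotation along RouteRef's spline.
; The Collision overlap damages the character, using a DoOnce that resets after two seconds to limit repeat hits.
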(event OnComponentBeginOverlap(Collision)
  (params (OverlappedComponent :type Primitive%20Component%20Object%20Reference) (OtherActor :type Actor%20Object%20Reference) (OtherComp :type Primitive%20Component%20Object%20Reference) (OtherBodyIndex :type Integer) (bFromSweep :type Boolean) (SweepResult :type Hit%20Result%20Structure%20%28by%20ref%29))
  ;[1 1 1] Damage
  (bind _asfirst_person_character (Utilities|Casting|CastToFirstPersonCharacter OtherActor))
  (Variables|Default|SetInVolume true)
  (Utilities|FlowControl|DoOnce false :!label _label
    (:Completed
      (Default|Damage _asfirst_person_character)
      (if (Variables|Default|GetInVolume)
        (Utilities|FlowControl|Delay 2.0)
        (goto _label Reset)))))

(event OnComponentBeginOverlap(StartMoveCheck)
  (params (OverlappedComponent :type Primitive%20Component%20Object%20Reference) (OtherActor :type Actor%20Object%20Reference) (OtherComp :type Primitive%20Component%20Object%20Reference) (OtherBodyIndex :type Integer) (bFromSweep :type Boolean) (SweepResult :type Hit%20Result%20Structure%20%28by%20ref%29))
  ;[1 1 1] Begin Moving
  (if (== OtherActor (Game|GetPlayerCharacter 0))
    (if (Variables|Default|GetIdolCollected)
      (Utilities|FlowControl|DoOnce false :!label _label
        (:Completed
          (CallFunction|MoveBoulder)
          (if (Variables|/Game/Level/Blueprints/Character/FirstPersonCharacter.FirstPersonCharacter_C|GetDeath (stale EventTick _asfirst_person_character))
            (goto _label Reset)))))))

(event Custom|MoveBoulder
  (bind _routeref (Variables|Default|GetRouteRef))
  (bind _boulderroute (Variables|/Game/Level/Blueprints/Traps/BP_Boulder_Route.BP_Boulder_Route_C|GetBoulderRoute _routeref))
  ;[1 1 1] Move Boulder
  (Audio|PlaySoundatLocation "/Game/Level/Audio/boulder_crumble.boulder_crumble" (Transformation|GetWorldLocation (Variables|Default|GetBoulder)) "0, 0, 0" 1.0 1.0 0.0 0 0 0)
  (Utilities|FlowControl|Delay (Variables|Default|GetDelay))
  (Components|Timeline|SetPlayRate (Variables|Default|GetBoulderMover) (/ 1.0 (Variables|Default|GetMoveSpeed)))
  (bind _alpha (Timeline|BoulderMover Play)
    (:Update
      (Variables|Default|SetAlpha _alpha)
      (Transformation|SetActorLocationAndRotation (Spline|GetLocationatDistanceAlongSpline _boulderroute (Math|Float|Lerp 0.0 (Spline|GetSplineLength _boulderroute) (Variables|Default|GetAlpha)) "World") (Spline|GetRotationatDistanceAlongSpline _boulderroute (Math|Float|Lerp 0.0 (Spline|GetSplineLength _boulderroute) (Variables|Default|GetAlpha)) "World")))))

(event EventTick
  (params (DeltaSeconds :type Float%20%28single-precision%29))
  ;[1 1 1] Check if the idol has been collected
  (Utilities|FlowControl|Sequence
    (:then_0
      (bind _asfirst_person_character (Utilities|Casting|CastToFirstPersonCharacter (Game|GetPlayerCharacter 0)))
      (Variables|Default|SetIdolCollected (Variables|/Game/Level/Blueprints/Character/FirstPersonCharacter.FirstPersonCharacter_C|GetIdolCollected _asfirst_person_character)))))

(fn ConstructionScript)