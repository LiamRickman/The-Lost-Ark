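; BP_Log is a log trap that travels along a spline route and damages the first-person player on contact.
; If LogMoveTrue is set, BeginPlay starts a timeline with duration scaled by MoveSpeed, mapping its alpha to position and rotation along RouteRef's LogRoute spline.
; Collision overlap calls the character's Damage and sets InVolume.
; The following two-second Delay leads to nothing, so damage does not repeat during an overlap.
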(event OnComponentBeginOverlap(Collision)
  (params (OverlappedComponent :type Primitive%20Component%20Object%20Reference) (OtherActor :type Actor%20Object%20Reference) (OtherComp :type Primitive%20Component%20Object%20Reference) (OtherBodyIndex :type Integer) (bFromSweep :type Boolean) (SweepResult :type Hit%20Result%20Structure%20%28by%20ref%29))
  ;[1 1 1] Check if take damage
  (bind _asfirst_person_character (Utilities|Casting|CastToFirstPersonCharacter OtherActor))
  (Variables|Default|SetInVolume true)
  (Default|Damage _asfirst_person_character)
  (if (Variables|Default|GetInVolume)
    (Utilities|FlowControl|Delay 2.0)))

(event Custom|MoveLog
  (bind _routeref (Variables|Default|GetRouteRef))
  (bind _logroute (Variables|/Game/Level/Blueprints/Traps/BP_Log_Route.BP_Log_Route_C|GetLogRoute _routeref))
  ;[1 1 1] Move Log along spline
  (Components|Timeline|SetPlayRate (Variables|Default|GetLogMover) (/ 1.0 (Variables|Default|GetMoveSpeed)))
  (bind _alpha (Timeline|LogMover Play)
    (:Update
      (Variables|Default|SetAlpha _alpha)
      (Transformation|SetActorLocationAndRotation (Spline|GetLocationatDistanceAlongSpline _logroute (Math|Float|Lerp 0.0 (Spline|GetSplineLength _logroute) (Variables|Default|GetAlpha)) "World") (Spline|GetRotationatDistanceAlongSpline _logroute (Math|Float|Lerp 0.0 (Spline|GetSplineLength _logroute) (Variables|Default|GetAlpha)) "World")))))

(event EventBeginPlay
  ;[1 1 1] Start log moving
  (if (Variables|Default|GetLogMoveTrue)
    (CallFunction|MoveLog)))

(fn ConstructionScript)