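; BP_Rope is a swingable rope trap actor that the player grabs on touch.
; Collision overlap sends a grab-rope message to player actors, passing itself.
; AddSwingingForce pushes CableEnd as an acceleration, limited by its height relative to the actor.
; While the player is not hanging, Tick sets CableEnd's world location to the relative location saved at BeginPlay.
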(event OnComponentBeginOverlap(Collision)
  (params (OverlappedComponent :type Primitive%20Component%20Object%20Reference) (OtherActor :type Actor%20Object%20Reference) (OtherComp :type Primitive%20Component%20Object%20Reference) (OtherBodyIndex :type Integer) (bFromSweep :type Boolean) (SweepResult :type Hit%20Result%20Structure%20%28by%20ref%29))
  ;[1 1 1] Attach Player to Rope
  (bind _yes_no (Class|BPIPlayer|IsPlayer(Message) OtherActor))
  (if _yes_no
    (Class|BPIPlayer|GrabRope(Message) OtherActor self)))

(event Custom|Add%20Swinging%20Force
  (params (Swing%20Force :type Vector))
  (bind _returnvalue (* Swing%20Force 5e+02))
  ;[1 1 1] Add Swinging Force
  (if (< (- (.z (Transformation|GetWorldLocation (Variables|Default|GetCable%20End))) (.z (Transformation|GetActorLocation))) 5e+02)
    (Physics|AddForce (Variables|Default|GetCable%20End) (Math|Vector|MakeVector (.x _returnvalue) (.y _returnvalue) (.z _returnvalue)) "None" true)))

(event EventTick
  (params (DeltaSeconds :type Float%20%28single-precision%29))
  ;[1 1 1] Update cable if player is hanging
  (bind _asfirst_person_character (Utilities|Casting|CastToFirstPersonCharacter (Game|GetPlayerCharacter 0)))
  (if (not (Variables|/Game/Level/Blueprints/Character/FirstPersonCharacter.FirstPersonCharacter_C|GetHanging _asfirst_person_character))
    (Transformation|SetWorldLocation (Variables|Default|GetCable%20End) (Variables|Default|GetCableLocation) false false)))

(event EventBeginPlay
  ;[1 1 1] Set Location
  (Variables|Default|SetCableLocation (Variables|/Script/Engine.SceneComponent|GetRelativeLocation (Variables|Default|GetCable%20End))))

(fn ConstructionScript)