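; Cobweb trap that the player can temporarily clear with the Interact input while standing inside its InRange volume.
; Overlap toggles input and the CanDestroy flag; a DoOnce throttles presses with a timed reset.
; A successful press plays the FadeInAndOut timeline, meant to drive Transparency on a dynamic material, and disables collision shortly after.
; After a longer delay, the timeline reverses and collision returns.
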(event OnComponentBeginOverlap(InRange)
  (params (OverlappedComponent :type Primitive%20Component%20Object%20Reference) (OtherActor :type Actor%20Object%20Reference) (OtherComp :type Primitive%20Component%20Object%20Reference) (OtherBodyIndex :type Integer) (bFromSweep :type Boolean) (SweepResult :type Hit%20Result%20Structure%20%28by%20ref%29))
  ;[1 1 1] Check if in range of cobweb
  (if (== OtherActor (Game|GetPlayerCharacter 0))
    (Variables|Default|SetCanDestroy true)
    (Input|EnableInput (Game|GetPlayerController 0))))

(event OnComponentEndOverlap(InRange)
  (params (OverlappedComponent :type Primitive%20Component%20Object%20Reference) (OtherActor :type Actor%20Object%20Reference) (OtherComp :type Primitive%20Component%20Object%20Reference) (OtherBodyIndex :type Integer))
  ;[1 1 1] Check if in range of cobweb
  (if (== OtherActor (Game|GetPlayerCharacter 0))
    (Variables|Default|SetCanDestroy false)
    (Input|DisableInput (Game|GetPlayerController 0))))

(event EventBeginPlay
  ;[1 1 1] Set up cobweb material
  (bind _returnvalue (Rendering|Material|CreateDynamicMaterialInstance (Variables|Default|GetCobweb) 0 "/Game/Level/Materials/M_Cobweb.M_Cobweb" "None" :!class /Script/Engine.PrimitiveComponent)))

(event Input|ActionEvents|InputActionInteract
  (params (Key :type Key%20Structure :default "None"))
  (bind _cobweb (Variables|Default|GetCobweb))
  (bind _fadeinandout (Variables|Default|GetFadeInAndOut))
  ;[1 1 1] Interact with cobweb
  (:Pressed
    (Utilities|FlowControl|DoOnce false :!label _label
      (:Completed
        (Utilities|FlowControl|Sequence
          (:then_0
            (Utilities|FlowControl|Delay 6.0)
            (goto _label Reset))
          (:then_1
            (if (Variables|Default|GetCanDestroy)
              (Utilities|FlowControl|Sequence
                (:then_0
                  (Audio|Components|Audio|Play _fadeinandout)
                  (Utilities|FlowControl|Delay 0.75)
                  (Collision|SetCollisionEnabled _cobweb "NoCollision"))
                (:then_1
                  (Utilities|FlowControl|Delay 1e+01)
                  (Utilities|String|Reverse _fadeinandout)
                  (Collision|SetCollisionEnabled _cobweb "QueryAndPhysics"))))))))))

(fn ConstructionScript)