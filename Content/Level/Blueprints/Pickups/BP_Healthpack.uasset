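; Health pickup Blueprint that grants the player one extra life.
; When a FirstPersonCharacter overlaps the Sphere trigger with fewer than five Lives, it increments that character's Lives.
; The pickup is consumed by disabling collision and hiding the Health component and PointLight rather than destroying the actor, with no respawn logic.
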(event OnComponentBeginOverlap(Sphere)
  (params (OverlappedComponent :type Primitive%20Component%20Object%20Reference) (OtherActor :type Actor%20Object%20Reference) (OtherComp :type Primitive%20Component%20Object%20Reference) (OtherBodyIndex :type Integer) (bFromSweep :type Boolean) (SweepResult :type Hit%20Result%20Structure%20%28by%20ref%29))
  (bind _health (Variables|Default|GetHealth))
  (bind _asfirst_person_character (Utilities|Casting|CastToFirstPersonCharacter OtherActor))
  (if (not (>= (Variables|/Game/Level/Blueprints/Character/FirstPersonCharacter.FirstPersonCharacter_C|GetLives _asfirst_person_character) 5))
    (Collision|SetCollisionEnabled _health "NoCollision")
    (Rendering|SetVisibility _health false false)
    (Variables|/Game/Level/Blueprints/Character/FirstPersonCharacter.FirstPersonCharacter_C|SetLives _asfirst_person_character (+ (Variables|/Game/Level/Blueprints/Character/FirstPersonCharacter.FirstPersonCharacter_C|GetLives _asfirst_person_character) 1))))

(fn ConstructionScript)