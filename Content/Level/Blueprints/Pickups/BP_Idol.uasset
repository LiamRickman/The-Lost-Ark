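; BP_Idol is the temple idol pickup that the first-person character collects to start the escape.
; When the character overlaps its Sphere, it disables collision on the idol and sphere and hides the idol mesh and point light.
; It then sets IdolCollected on the character and drives that character's subtitle variables to show a collapse warning, hiding it after a short delay.
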(event OnComponentBeginOverlap(Sphere)
  (params (OverlappedComponent :type Primitive%20Component%20Object%20Reference) (OtherActor :type Actor%20Object%20Reference) (OtherComp :type Primitive%20Component%20Object%20Reference) (OtherBodyIndex :type Integer) (bFromSweep :type Boolean) (SweepResult :type Hit%20Result%20Structure%20%28by%20ref%29))
  (bind _idol (Variables|Default|GetIdol))
  (bind _asfirst_person_character (Utilities|Casting|CastToFirstPersonCharacter OtherActor))
  (Collision|SetCollisionEnabled _idol "NoCollision")
  (Rendering|SetVisibility _idol false false)
  (Variables|/Game/Level/Blueprints/Character/FirstPersonCharacter.FirstPersonCharacter_C|SetIdolCollected _asfirst_person_character true)
  (Variables|/Game/Level/Blueprints/Character/FirstPersonCharacter.FirstPersonCharacter_C|SetSubtitleText _asfirst_person_character "The temple is collapsing! Get out of there!")
  (Variables|/Game/Level/Blueprints/Character/FirstPersonCharacter.FirstPersonCharacter_C|SetSubtitleVisibility _asfirst_person_character true)
  (Utilities|FlowControl|Delay 5.0)
  (Variables|/Game/Level/Blueprints/Character/FirstPersonCharacter.FirstPersonCharacter_C|SetSubtitleVisibility _asfirst_person_character false))

(fn ConstructionScript)